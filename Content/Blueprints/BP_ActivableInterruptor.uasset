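; BP_ActivableInterruptor is a switch that stays inert until a main interruptor event enables it.
; On BeginPlay it binds Activate through InterruptorEventEmitter; Activate sets IsOn, unbinds all events from that emitter's main interruptor and shows the active material.
; While on, third-person character overlap sends ActivateMessage to InterfacesToActivate entries implementing BPI_InterruptorActivable and shows the used material.
; Leaving the box restores the active material, so it can retrigger.
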(event `self.ReceiveBeginPlay`
  (add `/Game/Blueprints/BP_InterruptorEventEmitter.MainInteruptor` (`self.InterruptorEventEmitter`) (delegate `Activate`)))

(event `Activate`
  (clear `/Game/Blueprints/BP_InterruptorEventEmitter.MainInteruptor` (`self.InterruptorEventEmitter`))
  (set `self.IsOn` true)
  (`PrimitiveComponent.SetMaterial` (`self.Cube`) 0 "/Game/Materials/MI_ActiveInterruptor.MI_ActiveInterruptor"))

(event `self.Box.OnComponentBeginOverlap`
  (params (OverlappedComponent :type "PrimitiveComponent Object Reference") (OtherActor :type "Actor Object Reference") (OtherComp :type "PrimitiveComponent Object Reference") (OtherBodyIndex :type Integer) (bFromSweep :type Boolean) (SweepResult :type "HitResult Structure (by ref)"))
  (cast `/Game/ThirdPerson/Blueprints/BP_ThirdPersonCharacter` OtherActor)
  (if (`self.IsOn`)
    (`self.CallInterfacesActivate`)
    (`PrimitiveComponent.SetMaterial` (`self.Cube`) 0 "/Game/Materials/MI_UsedInterruptor.MI_UsedInterruptor")))

(event `self.Box.OnComponentEndOverlap`
  (params (OverlappedComponent :type "PrimitiveComponent Object Reference") (OtherActor :type "Actor Object Reference") (OtherComp :type "PrimitiveComponent Object Reference") (OtherBodyIndex :type Integer))
  (cast `/Game/ThirdPerson/Blueprints/BP_ThirdPersonCharacter` OtherActor)
  (if (`self.IsOn`)
    (`PrimitiveComponent.SetMaterial` (`self.Cube`) 0 "/Game/Materials/MI_ActiveInterruptor.MI_ActiveInterruptor")))

(fn `CallInterfacesActivate`
  (for _array_element (`self.InterfacesToActivate`)
    (if (`KismetSystemLibrary.DoesImplementInterface` _array_element "/Game/Blueprints/BPI_InterruptorActivable.BPI_InterruptorActivable_C")
      (message `/Game/Blueprints/BPI_InterruptorActivable.Activate` _array_element))))

(fn `UserConstructionScript`)