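; BP_DoorPuzzle is a toggleable door that forms part of a light puzzle.
; ChangeState snaps the door between closed and a 90-degree yaw, using its current yaw as the state, and adjusts the open-door count on LightPuzzle.
; Activate toggles the door and then asks LightPuzzle to check completion.
; Doors flagged StartOpen toggle on BeginPlay without that check.
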(event `self.ReceiveBeginPlay`
  (if (`self.StartOpen`)
    (`self.ChangeState`)))

(event `/Game/Blueprints/BPI_InterruptorActivable.Activate`
  (`self.ChangeState`)
  (`/Game/Blueprints/BP_LightPuzzle.CheckCompletion` (`self.LightPuzzle`)))

(fn `ChangeState`
  (bind _door (`self.Door`))
  (bind (_relativerotation_roll _relativerotation_pitch _relativerotation_yaw) (`KismetMathLibrary.BreakRotator` (`SceneComponent.RelativeRotation` _door)))
  (bind _opendoors (`/Game/Blueprints/BP_LightPuzzle.OpenDoors` (`self.LightPuzzle`)))
  (if (> _relativerotation_yaw 0.0)
    (`SceneComponent.K2_SetRelativeRotation` :`self` _door)
    (`/Engine/EditorBlueprintResources/StandardMacros.DecrementInt` _opendoors)
    (else
      (`SceneComponent.K2_SetRelativeRotation` _door (struct :`Yaw` 90.0) false false)
      (`/Engine/EditorBlueprintResources/StandardMacros.IncrementInt` _opendoors))))

(fn `UserConstructionScript`)